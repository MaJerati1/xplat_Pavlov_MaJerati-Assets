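; SkinBox is a Pavlov trigger actor that applies its configured skin to a player whose pawn overlaps it.
; On BeginPlay it sets the volume material and displays the skin name on a TextRender through ReplicateText.
; Overlaps are handled on the authority, setting the skin through the player proxy.
; Boxes flagged SpecialSkinBox only work for a hardcoded whitelist of player names.
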(event Custom|ReplicateText
  (Rendering|Components|TextRender|SetText (Variables|Default|GetTextRender) (stale EventBeginPlay _output_get)))

(event EventBeginPlay
  (Rendering|Material|SetMaterial (Variables|Default|GetSkinVolume) 0 (Variables|Default|GetMaterialForVolume))
  (bind _output_get (Variables|Default|SetTextRep (Utilities|Text|ToText(Name) (Variables|Default|GetSkin))))
  (CallFunction|ReplicateText))

(event Collision|EventActorBeginOverlap
  (params (OtherActor :type Actor%20Object%20Reference))
  (Networking|SwitchHasAuthority
    (:Authority
      (bind _aspawn (Utilities|Casting|CastToPawn OtherActor))
      (bind _playerstatus (Class|PavlovProxyStatics|GetPavlovPlayerStatusbyPawn _aspawn))
      (if (Variables|Default|GetSpecialSkinBox)
        (if (Utilities|Array|ContainsItem (Utilities|Array|MakeArray "MaJerati" "SrryItsJay" "kingsrocky" "RickyGrimesPrime" "MrFlintlock" "dragonflamz" "Entertainmentz" "Wmini20" "D4Y13") (PlayerState|GetPlayerName (.PlayerState (Utilities|Struct|BreakPavlovPlayerStatus _playerstatus))))
          (Class|PavlovPlayerProxy|SetPlayerSkin (Class|PavlovLibrary|GetPlayerProxy _aspawn) (Variables|Default|GetSkin) :!label _label))
        (else
          (goto _label))))))

(fn ConstructionScript)

(fn OnRepTextRep)