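; BP_TestItemSpawner is a debug-map actor that spawns a configurable Pavlov item for the player who grabs its interact box.
; A client grab replicates to the server through the hand proxy.
; The server resolves the player's state from their pawn and calls game logic to spawn the named item with a magazine for their dominant hand, logging the result.
; The construction script sets the label text from a variable.
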(event OnInteractBoxClient(Pavlov_InteractBox)
  (params (InteractType :type EInteractType%20Enum :default "Grabbed") (HandProxy :type Pavlov%20Hand%20Proxy%20Object%20Reference) (InteractBox :type Pavlov%20Interact%20Box%20Object%20Reference))
  (if (Utilities|Enum|Equal(Enum) InteractType "Grabbed")
    (Class|PavlovHandProxy|ReplicateInteractServer HandProxy InteractType InteractBox)
    (Class|PavlovLibrary|LogtoConsole "Replicate Interact" false)
    (else
      (Class|PavlovLibrary|LogtoConsole "Replicate Interact failed, trigger" false))))

(event OnInteractBoxServer(Pavlov_InteractBox)
  (params (InteractType :type EInteractType%20Enum :default "Grabbed") (HandProxy :type Pavlov%20Hand%20Proxy%20Object%20Reference) (InteractBox :type Pavlov%20Interact%20Box%20Object%20Reference))
  (bind _itemname (Variables|Default|GetItemName))
  (bind _playerstatus (Class|PavlovProxyStatics|GetPavlovPlayerStatusbyPawn (Class|PavlovPlayerProxy|GetPawn (Class|PavlovHandProxy|GetPlayerProxy HandProxy))))
  (Class|PavlovGameLogic|SpawnItem (Class|PavlovLibrary|GetGameLogic) (Utilities|Struct|MakePavlovItemSpawnParams _itemname (.PlayerState (Utilities|Struct|BreakPavlovPlayerStatus _playerstatus)) (Variables|/Script/PavlovProxy.Pavlov_HandProxy|GetbDominantHand HandProxy) false 0 false "0.000000,0.000000,0.000000|0.000000,0.000000,-0.000000|1.000000,1.000000,1.000000" true false))
  (Class|PavlovLibrary|LogtoConsole (Utilities|String|Append "Spawn Item " (Utilities|String|ToString(Name) _itemname)) false))

(event EventBeginPlay)

(event Collision|EventActorBeginOverlap
  (params (OtherActor :type Actor%20Object%20Reference)))

(event EventTick
  (params (DeltaSeconds :type Float%20%28single-precision%29)))

(fn ConstructionScript
  (Rendering|Components|TextRender|SetText (Variables|Default|GetTextRender) (Variables|Default|GetText)))