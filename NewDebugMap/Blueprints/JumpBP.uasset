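; JumpBP is an actor that adds a jump to the local Pavlov player, triggered by pressing the right thumbstick.
; On BeginPlay it enables input for player controller 0, except on a dedicated server.
; A jump requires the player to be neither crouching nor falling, then launches the character upward with a slight forward push.
; Players with the "mayro" skin get double the launch height.
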(event Custom|StartJump
  (bind _returnvalue (Game|GetPlayerCharacter 0))
  (bind _returnvalue_2 (Transformation|GetActorForwardVector _returnvalue))
  (bind _returnvalue_3 (* _returnvalue_2 1e+01))
  (bind (_x _y) (Math|Vector|BreakVector _returnvalue_3))
  (bind _playerstatus (Class|PavlovProxyStatics|GetPavlovPlayerStatus (Variables|/Script/Engine.Controller|GetPlayerState (Game|GetPlayerController 0))))
  (if (not (.bCrouching (Utilities|Struct|BreakPavlovPlayerStatus _playerstatus)))
    (if (not (AI|Components|NavMovement|IsFalling (Variables|/Script/Engine.Character|GetCharacterMovement _returnvalue)))
      (if (== (Class|PavlovPlayerProxy|GetPlayerSkin (Class|PavlovLibrary|GetPlayerProxy (.Pawn (Utilities|Struct|BreakPavlovPlayerStatus _playerstatus)))) "mayro")
        (Variables|Default|SetJumpingHeight 4e+03)
        (else
          (Variables|Default|SetJumpingHeight 2e+03)))
      (Character|LaunchCharacter (Game|GetPlayerCharacter 0) (Math|Vector|MakeVector _x _y (Variables|Default|GetJumpingHeight)) false true))))

(event EventBeginPlay
  (if (not (Networking|IsDedicatedServer))
    (Input|EnableInput (Game|GetPlayerController 0))))

(event Collision|EventActorBeginOverlap
  (params (OtherActor :type Actor%20Object%20Reference)))

(event Input|ActionEvents|InputActionThumbstickPressRight
  (params (Key :type Key%20Structure))
  (:Pressed
    (CallFunction|StartJump)))

(fn ConstructionScript
  (bind _outactors (Actor|GetAllActorsOfClass "/Script/PavlovProxy.Pavlov_GameLogic")))