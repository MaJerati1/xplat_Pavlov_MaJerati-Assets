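; Loot spawner Blueprint that configures its parent spawner with either a specific item or a randomized list of items chosen through enums.
; The construction script converts enum selections into SpawnList names and looks up DTT_LootSpawnerWM to set an editor preview mesh.
; It also sets the preview's hidden-in-game state and copies spawner type, wait times and attachment settings into spawner variables.
; BeginPlay rebuilds and shuffles the list when random mode is on.
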(event EventBeginPlay
  (if (Variables|LSWCM|RandomLoot|GetbUse/CreateRandomList?)
    (Utilities|Array|Clear (Variables|Default|GetSpawnList))
    (for _array_element (Variables|LSWCM|RandomLoot|GetRandomLootList)
      (Utilities|Array|Add (Variables|Default|GetSpawnList) (Utilities|String|EnumtoString _array_element))
      (Utilities|Array|Shuffle (Variables|Default|GetSpawnList)))))

(fn ConstructionScript
  (bind _spawnlist (Variables|Default|GetSpawnList))
  (bind _item (Variables|Default|GetItem))
  (bind _bhideingameview (Variables|LSWCM|GetbHideInGameView))
  (Utilities|FlowControl|Sequence
    (:then_0
      ;[1 1 1] Make Random List - Change model to one of the Random Loot List
      (if (Variables|LSWCM|RandomLoot|GetbUse/CreateRandomList?)
        (Utilities|Array|Clear (Variables|Default|GetSpawnList))
        (for _array_element (Variables|LSWCM|RandomLoot|GetRandomLootList)
          (Utilities|Array|Add (Variables|Default|GetSpawnList) (Utilities|String|EnumtoString _array_element))
          (Utilities|Array|Shuffle _spawnlist)
          (bind _returnvalue (Utilities|GetDataTableRow "/Game/Blueprints/DTT_LootSpawnerWM.DTT_LootSpawnerWM" (Utilities|String|StringToName (Utilities|Array|Get(acopy) _spawnlist)))
            (:then
              (Components|StaticMesh|SetStaticMesh (Variables|Default|GetItem) (.staticmesh _returnvalue)))))
        (else
          ;[1 1 1] Set Unique Item - Spawn a specific item
          (if (> (Variables|LSWCM|GetLootToSpawn) 0)
            (Utilities|Array|Clear (Variables|Default|GetSpawnList))
            (Utilities|Array|AddUnique (Variables|Default|GetSpawnList) (Utilities|String|EnumtoString (Variables|LSWCM|GetLootToSpawn)))
            (else
              (|CallParentFunction))))))
    (:then_1
      ;[1 1 1] Set Visible Editor Model - Set the Visible Model based on last selected Item - Editor Only
      (bind _returnvalue_2 (Utilities|GetDataTableRow "/Game/Blueprints/DTT_LootSpawnerWM.DTT_LootSpawnerWM" (Utilities|String|StringToName (Utilities|String|EnumtoString (Variables|LSWCM|GetLootToSpawn))))
        (:then
          (Components|StaticMesh|SetStaticMesh (Variables|Default|GetItem) (.staticmesh _returnvalue_2)))))
    (:then_2
      ;[1 1 1] Hide in Game View - Toggle the Visible Model in Game View (G) - Editor Only - For Screenshoting purposes
      (Utilities|FlowControl|FlipFlop
        (:A
          (Development|SetHiddeninGame _item _bhideingameview false))
        (:B
          (Development|SetHiddeninGame _item _bhideingameview false))))
    (:then_3
      ;[1 1 1] Move Loot Spawner Settings in to LSWCM - Set Spawner Type - Easier to Use
      (Variables|Default|SetSpawnerType (Math|Conversions|ToInteger(Byte) (Variables|LSWCM|GetLootSpawnerType)))
      (Variables|Default|SetMinSpawnTime (Variables|LSWCM|GetMinimumWaitTimeToSpawn))
      (Variables|Default|SetMaxSpawnTime (Variables|LSWCM|GetMaximumWaitTimeToSpawn))
      (Variables|Default|SetSpawnWithoutAttachments (Variables|LSWCM|GetbSpawnWithoutAttachments)))
    (:then_4
      (|CallParentFunction))))