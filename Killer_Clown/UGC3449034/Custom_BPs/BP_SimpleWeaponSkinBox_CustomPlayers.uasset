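; Pavlov trigger box that reskins weapons and magazines overlapping it, optionally only for listed players.
; With UsePlayerIDS on, the owning pawn's player name must appear in PlayerIDs.
; Overlapping actors are matched by class-name substring against GunID or MagazineID and stored in GUN or MAG.
; Those variables' RepNotifies apply the Slot1 and Slot2 materials to mesh components; SwitchSlots reverses the order for guns only.
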(event OnComponentBeginOverlap(Box)
  (params (OverlappedComponent :type Primitive%20Component%20Object%20Reference) (OtherActor :type Actor%20Object%20Reference) (OtherComp :type Primitive%20Component%20Object%20Reference) (OtherBodyIndex :type Integer) (bFromSweep :type Boolean) (SweepResult :type Hit%20Result%20Structure%20%28by%20ref%29))
  (bind _returnvalue (Utilities|GetClass OtherActor))
  (bind _returnvalue_2 (Utilities|GetClassDisplayName _returnvalue))
  (if (Variables|Default|GetUsePlayerIDS?)
    (bind _aspawn (Utilities|Casting|CastToPawn (Components|GetOwner OtherActor)))
    (bind _playerstatus (Class|PavlovProxyStatics|GetPavlovPlayerStatusbyPawn _aspawn))
    (if (Utilities|Array|ContainsItem (Variables|Default|GetPlayerIDs) (PlayerState|GetPlayerName (.PlayerState (Utilities|Struct|BreakPavlovPlayerStatus _playerstatus))))
      (if (Utilities|String|Contains _returnvalue_2 (Variables|Default|GetGun%20ID)) :!label _label
        (Variables|Default|SetGUN OtherActor)
        (elif (Utilities|String|Contains _returnvalue_2 (Variables|Default|GetMagazine%20ID))
          (Variables|Default|SetMAG OtherActor))))
    (else
      (goto _label))))

(fn ConstructionScript)

(fn OnRepGUN
  (bind _gun (Variables|Default|GetGUN))
  (bind _slot1 (Variables|Default|GetSlot1))
  (bind _slot2 (Variables|Default|GetSlot2))
  (bind _returnvalue (Actor|GetComponentsByClass _gun "/Script/Engine.MeshComponent"))
  (if (Variables|Default|GetSwitch%20Slots?)
    (Rendering|Material|SetMaterial _returnvalue 1 _slot1)
    (Rendering|Material|SetMaterial _returnvalue 0 _slot2)
    (else
      (Rendering|Material|SetMaterial _returnvalue 0 _slot1)
      (Rendering|Material|SetMaterial _returnvalue 1 _slot2))))

(fn OnRepMAG
  (bind _mag (Variables|Default|GetMAG))
  (bind _returnvalue (Actor|GetComponentsByClass _mag "/Script/Engine.MeshComponent"))
  (Rendering|Material|SetMaterial _returnvalue 0 (Variables|Default|GetSlot1))
  (Rendering|Material|SetMaterial _returnvalue 1 (Variables|Default|GetSlot2)))